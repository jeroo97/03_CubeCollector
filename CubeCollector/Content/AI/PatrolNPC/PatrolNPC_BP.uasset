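; Patrol NPC drone that shows its AI state to the player through chase and search signs and a health bar.
; BeginPlay stores the FirstPersonCharacter and links the DroneHealthBar widget back to this drone.
; Tick polls the Blackboard for CanSeePlayer and IsInvestigating to toggle the signs, updating the search sign only while the player is unseen.
; Losing possession plays a glass-break sound at its location.
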(event EventBeginPlay
  (bind _returnvalue (Actor|GetActorOfClass "/Game/FirstPersonCPP/Blueprints/FirstPersonCharacter.FirstPersonCharacter_C"))
  (Class|PatrolNPC|SetCharacter _returnvalue)
  (CallFunction|InitialiseHealthBarWidget))

(event EventUnpossessed
  (params (OldController :type Controller%20Object%20Reference))
  (Audio|PlaySoundatLocation "/Game/Sounds/Glass_Break-stephan_schutze-958181291.Glass_Break-stephan_schutze-958181291" (Transformation|GetActorLocation) "0, 0, 0" 2.0 1.0 0.0 0 0 0))

(event EventTick
  (params (DeltaSeconds :type Float%20%28single-precision%29))
  (bind _returnvalue (AI|GetBlackboard 0))
  (bind _returnvalue_2 (AI|GetBlackboard 0))
  (Utilities|IsValid _returnvalue_2
    (:Is%20Valid
      (if (ScalableFloat|GetValueasBool _returnvalue_2 (Utilities|Name|MakeLiteralName "CanSeePlayer"))
        (Rendering|SetVisibility (Variables|Default|GetChaseSign) true false)
        (else
          (Rendering|SetVisibility (Variables|Default|GetChaseSign) false false)
          (Utilities|IsValid _returnvalue
            (:Is%20Valid
              (if (ScalableFloat|GetValueasBool _returnvalue (Utilities|Name|MakeLiteralName "IsInvestigating"))
                (Rendering|SetVisibility (Variables|Default|GetSearchSign) true false)
                (else
                  (Rendering|SetVisibility (Variables|Default|GetSearchSign) false false))))))))))

(fn ConstructionScript)

(fn InitialiseHealthBarWidget
  (bind _asdrone_health_bar (Utilities|Casting|CastToDroneHealthBar (UserInterface|GetUserWidgetObject (Variables|Default|GetHealthBar))))
  (Variables|/Game/UI/DroneHealthBar.DroneHealthBar_C|SetMy%20Drone _asdrone_health_bar self)
  (return))