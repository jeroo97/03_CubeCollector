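; Runner NPC pawn that flees from the player and, when caught, damages every patrol NPC.
; Each Tick it sets the RunningAway blackboard key according to whether the player is within a fixed distance, leaving movement to the AI.
; A capsule overlap with the player, matched by hard-coded object name, calls TakeHealth on all PatrolNPC_BP actors.
; DestroyActor runs inside that loop, so the runner removes itself only if patrols exist.
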(event OnComponentBeginOverlap(CapsuleComponent)
  (params (OverlappedComponent :type Primitive%20Component%20Object%20Reference) (OtherActor :type Actor%20Object%20Reference) (OtherComp :type Primitive%20Component%20Object%20Reference) (OtherBodyIndex :type Integer) (bFromSweep :type Boolean) (SweepResult :type Hit%20Result%20Structure%20%28by%20ref%29))
  (if (Utilities|Enum|Equal(Enum) (Utilities|GetObjectName OtherActor) "FirstPersonCharacter_C_0")
    (Development|PrintString "Inflicting damage to all patrols")
    (bind _outactors (Actor|GetAllActorsOfClass "/Game/AI/PatrolNPC/PatrolNPC_BP.PatrolNPC_BP_C"))
    (for _array_element _outactors
      (Class|PatrolNPC|TakeHealth _array_element 2)
      (Actor|DestroyActor))))

(event EventBeginPlay)

(event Collision|EventActorBeginOverlap
  (params (OtherActor :type Actor%20Object%20Reference)))

(event EventTick
  (params (DeltaSeconds :type Float%20%28single-precision%29))
  (bind _returnvalue (Pawn|GetController))
  (if (< (Transformation|GetDistanceTo self (Game|GetPlayerCharacter 0)) 2e+03)
    (AI|Components|Blackboard|SetValueasBool (AI|GetBlackboard _returnvalue) (Utilities|Name|MakeLiteralName "RunningAway") true)
    (else
      (AI|Components|Blackboard|SetValueasBool (AI|GetBlackboard _returnvalue) (Utilities|Name|MakeLiteralName "RunningAway") false))))

(fn ConstructionScript)