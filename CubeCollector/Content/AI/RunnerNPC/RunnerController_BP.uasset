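; AI controller for the Runner NPC that runs its behavior tree on BeginPlay and passes perception results to the Blackboard.
; Target perception updates for the FirstPersonCharacter set CanSeePlayer from whether the stimulus was successfully sensed.
; General perception updates write TargetLocation from stimuli tagged "Sight" on any updated actor, without filtering for the player.
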(event OnTargetPerceptionUpdated(AIPerception)
  (params (Actor :type Actor%20Object%20Reference) (Stimulus :type AI%20Stimulus%20Structure))
  (Utilities|Casting|CastToFirstPersonCharacter Actor)
  (AI|Components|Blackboard|SetValueasBool (AI|GetBlackboard 0) (Utilities|Name|MakeLiteralName "CanSeePlayer") (.bSuccessfullySensed (Utilities|Struct|BreakAIStimulus Stimulus))))

(event OnPerceptionUpdated(AIPerception)
  (params (UpdatedActors :type Array%20of%20Actor%20Object%20References))
  (for _array_element UpdatedActors
    (bind _info (Class|AIPerceptionComponent|GetActorsPerception (Variables|Default|GetAIPerception) _array_element))
    (for _array_element_2 (.lastsensedstimuli _info)
      (if (Utilities|Name|Equal(Name) (.Tag (Utilities|Struct|BreakAIStimulus _array_element_2)) "Sight")
        (AI|Components|Blackboard|SetValueasVector (AI|GetBlackboard 0) (Utilities|Name|MakeLiteralName "TargetLocation") (.StimulusLocation (Utilities|Struct|BreakAIStimulus _array_element_2)))))))

(event EventBeginPlay
  (AI|RunBehaviorTree "/Game/AI/RunnerNPC/RunnerNPC_BT.RunnerNPC_BT"))

(fn ConstructionScript)